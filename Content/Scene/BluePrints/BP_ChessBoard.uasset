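; BP_ChessBoard is a chess board actor that detects whether specific pieces are placed on three key points, apparently for a puzzle.
; Each KeyPoint component's begin-overlap passes its index and the overlapping actor to the shared ChessPlaced event.
; ChessPlaced compares that actor with the TargetActor entry at that index and sends the true/false result and index to the Game Instance through ChessFlgMessage.
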(event OnComponentBeginOverlap(KeyPoint0)
  (params (OverlappedComponent :type Primitive%20Component%20Object%20Reference) (OtherActor :type Actor%20Object%20Reference) (OtherComp :type Primitive%20Component%20Object%20Reference) (OtherBodyIndex :type Integer) (bFromSweep :type Boolean) (SweepResult :type Hit%20Result%20Structure%20%28by%20ref%29))
  ;[1 1 1] 床の当たり判定
  (CallFunction|ChessPlaced 0 OtherActor))

(event OnComponentBeginOverlap(KeyPoint1)
  (params (OverlappedComponent :type Primitive%20Component%20Object%20Reference) (OtherActor :type Actor%20Object%20Reference) (OtherComp :type Primitive%20Component%20Object%20Reference) (OtherBodyIndex :type Integer) (bFromSweep :type Boolean) (SweepResult :type Hit%20Result%20Structure%20%28by%20ref%29))
  ;[1 1 1] 床の当たり判定
  (CallFunction|ChessPlaced 1 OtherActor))

(event OnComponentBeginOverlap(KeyPoint2)
  (params (OverlappedComponent :type Primitive%20Component%20Object%20Reference) (OtherActor :type Actor%20Object%20Reference) (OtherComp :type Primitive%20Component%20Object%20Reference) (OtherBodyIndex :type Integer) (bFromSweep :type Boolean) (SweepResult :type Hit%20Result%20Structure%20%28by%20ref%29))
  ;[1 1 1] 床の当たり判定
  (CallFunction|ChessPlaced 2 OtherActor))

(event Custom|ChessPlaced
  (params (Number :type Integer) (OtherActor :type Actor%20Object%20Reference))
  ;[1 1 1] オブジェクトがあっていたらフラグをTrue
  (Class|BPIEvent|ChessFlg(Message) (Game|GetGameInstance) (== (Utilities|Array|Get(acopy) (Variables|Default|GetTargetActor) Number) OtherActor) Number))

(event EventBeginPlay)

(event Collision|EventActorBeginOverlap
  (params (OtherActor :type Actor%20Object%20Reference)))

(event EventTick
  (params (DeltaSeconds :type Float%20%28single-precision%29)))

(fn ConstructionScript)