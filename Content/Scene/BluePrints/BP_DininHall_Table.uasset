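; Dining hall table placement check that tracks whether the correct object sits in its dish area, apparently for a puzzle.
; Box overlap events compare the entering or leaving actor to TargetActor and report to the GameInstance via ObjectFlgMessage, keyed by TableNum.
; Any entering actor sets the flag to the match result, so a wrong one sends false, while only the target leaving clears it.
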(event OnComponentBeginOverlap(Box)
  (params (OverlappedComponent :type Primitive%20Component%20Object%20Reference) (OtherActor :type Actor%20Object%20Reference) (OtherComp :type Primitive%20Component%20Object%20Reference) (OtherBodyIndex :type Integer) (bFromSweep :type Boolean) (SweepResult :type Hit%20Result%20Structure%20%28by%20ref%29))
  ;[1 1 1] 皿のあたり判定
  (CallFunction|ObjectPlaced (Variables|Default|GetTableNum) OtherActor))

(event OnComponentEndOverlap(Box)
  (params (OverlappedComponent :type Primitive%20Component%20Object%20Reference) (OtherActor :type Actor%20Object%20Reference) (OtherComp :type Primitive%20Component%20Object%20Reference) (OtherBodyIndex :type Integer))
  ;[1 1 1] ターゲットが外れた時
  (CallFunction|ObjectMissed (Variables|Default|GetTableNum) OtherActor))

(event Custom|ObjectPlaced
  (params (Number :type Integer) (otherActor :type Actor%20Object%20Reference))
  ;[1 1 1] オブジェクトがあっていたらフラグをTrue
  (Class|BPIEvent|ObjectFlg(Message) (Game|GetGameInstance) (== (Variables|Default|GetTargetActor) otherActor) Number))

(event Custom|ObjectMissed
  (params (number :type Integer) (otherActor :type Actor%20Object%20Reference))
  ;[1 1 1] エリアから外れたのがターゲットならFalse
  (if (== (Variables|Default|GetTargetActor) otherActor)
    (Class|BPIEvent|ObjectFlg(Message) (Game|GetGameInstance) false number)))

(event EventBeginPlay)

(event EventTick
  (params (DeltaSeconds :type Float%20%28single-precision%29)))

(fn ConstructionScript)