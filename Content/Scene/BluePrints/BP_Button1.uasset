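; BP_Button1 is a pressable button that appears to drive a door through an exposed flag.
; Each overlap on its Cylinder increments a press count, prints it modulo 8, and sets ButtonFlag when that value equals PushCnt.
; It then calls OnButtonDown on every press, and the DoorFlag function returns the flag.
; A timeline that would sway the actor along Y with a sine is never run.
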(event OnComponentBeginOverlap(Cylinder)
  (params (OverlappedComponent :type Primitive%20Component%20Object%20Reference) (OtherActor :type Actor%20Object%20Reference) (OtherComp :type Primitive%20Component%20Object%20Reference) (OtherBodyIndex :type Integer) (bFromSweep :type Boolean) (SweepResult :type Hit%20Result%20Structure%20%28by%20ref%29))
  (bind _output_get (Variables|Default|SetbuttonCnt (+ (Variables|Default|GetbuttonCnt) 1)))
  (bind _output_get_2 (Variables|Default|Setcnt (Math|Integer|%(Integer) _output_get 8)))
  (Development|PrintString (Utilities|String|ToString(Text) (Utilities|Text|ToText(Integer) _output_get_2)))
  (Variables|Default|SetbuttonFlag (== (Variables|Default|Getcnt) (Variables|Default|GetpushCnt)))
  (Default|CallOnButtonDown))

(event EventBeginPlay)

(event Collision|EventActorBeginOverlap
  (params (OtherActor :type Actor%20Object%20Reference)))

(event EventTick
  (params (DeltaSeconds :type Float%20%28single-precision%29)))

(fn ConstructionScript)

(fn DoorFlag
  (return (Variables|Default|GetbuttonFlag)))