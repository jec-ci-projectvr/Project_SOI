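; BP_CaveDoor is a cave door actor that rises when the mystery matching its own is passed through an OpenDoor interface event.
; It caches its root's world location on BeginPlay, then OpenDoor forwards to CheckAndOpen, which compares the Mystery values.
; On a match it plays a sound at that location and runs a timeline that lifts the actor along Z from the cached position.
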(event Custom|CheckAndOpen
  (params (mystery :type MysteryPlace%20Enum :default "NewEnumerator0"))
  (bind _beforepositon (Variables|Default|GetbeforePositon))
  ;[1 1 1] サーバーから扉を開く
  (if (Utilities|Enum|Equal(Enum) mystery (Variables|Default|Getmystery))
    (Audio|PlaySoundatLocation "/Game/Scene/Audio/SE/SE_StatueRotate.SE_StatueRotate" (Variables|Default|GetbeforePositon) "0, 0, 0" 1.0 1.0 0.0 0 0 0 0)
    (bind _door (Timeline|DoorAnimation Play)
      (:Update
        (Transformation|SetActorLocation (Math|Vector|MakeVector (.x _beforepositon) (.y _beforepositon) (+ (.z _beforepositon) (* _door 3e+02))) false false)))))

(event EventOpenDoor
  (params (mystery :type MysteryPlace%20Enum :default "NewEnumerator0"))
  ;[1 1 1] インターフェースから受け取り
  (CallFunction|CheckandOpen mystery))

(event Collision|EventActorBeginOverlap
  (params (OtherActor :type Actor%20Object%20Reference)))

(event EventTick
  (params (DeltaSeconds :type Float%20%28single-precision%29)))

(event EventBeginPlay
  ;[1 1 1] 最初の位置を取得
  (Variables|Default|SetbeforePositon (Transformation|GetWorldLocation (Variables|Default|GetDefaultSceneRoot))))

(fn ConstructionScript)