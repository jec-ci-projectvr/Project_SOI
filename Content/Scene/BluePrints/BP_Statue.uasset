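; BP_Statue is a puzzle statue that rotates when something overlaps its button.
; Each overlap plays two timelines at once: one yaws the base up to 45 degrees, the other moves the button vertically with its collision disabled.
; When the button timeline finishes, it restores collision and tells the game instance, by statue number, whether the base is within tolerance of its clear rotation.
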(event OnComponentBeginOverlap(Button)
  (params (OverlappedComponent :type Primitive%20Component%20Object%20Reference) (OtherActor :type Actor%20Object%20Reference) (OtherComp :type Primitive%20Component%20Object%20Reference) (OtherBodyIndex :type Integer) (bFromSweep :type Boolean) (SweepResult :type Hit%20Result%20Structure%20%28by%20ref%29))
  (bind _currentbuttonposition (Variables|Default|GetcurrentButtonPosition))
  (Variables|Default|SetcurrentSutatueRotation (Transformation|GetWorldRotation (Variables|Default|GetBase)))
  (Utilities|FlowControl|Sequence
    (:then_0
      (bind _rotation (Timeline|Rotate PlayFromStart)
        (:Update
          (Transformation|SetWorldRotation (Variables|Default|GetBase) (Math|Rotator|MakeRotator (.roll (Variables|Default|GetcurrentSutatueRotation)) (.pitch (Variables|Default|GetcurrentSutatueRotation)) (+ (.yaw (Variables|Default|GetcurrentSutatueRotation)) (* _rotation 45.0))) false false))))
    (:then_1
      (bind _新規track_0 (Timeline|ButtonDown PlayFromStart)
        (:Update
          (Transformation|SetWorldLocation (Variables|Default|GetButton) (Math|Vector|MakeVector (.x _currentbuttonposition) (.y _currentbuttonposition) (- (.z _currentbuttonposition) (* 1e+01 _新規track_0))) false false)
          (Collision|SetCollisionEnabled (Variables|Default|GetButton) "NoCollision"))
        (:Finished
          (Collision|SetCollisionEnabled (Variables|Default|GetButton) "QueryAndPhysics")
          (Class|BPIEvent|StatueFlg(Message) (Game|GetGameInstance) (Utilities|Operators|EqualEqual (Transformation|GetWorldRotation (Variables|Default|GetBase)) (Variables|Default|GeteventClearRotate) 1e+01) (Variables|Default|GetsutatueNum)))))))

(event EventBeginPlay
  (Variables|Default|SetcurrentButtonPosition (Transformation|GetWorldLocation (Variables|Default|GetButton))))

(event Collision|EventActorBeginOverlap
  (params (OtherActor :type Actor%20Object%20Reference)))

(event EventTick
  (params (DeltaSeconds :type Float%20%28single-precision%29)))

(fn ConstructionScript)