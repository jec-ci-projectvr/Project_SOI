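; BP_DininHall_CreamSliced is a dining hall prop, apparently a plated cream slice, with a name label and an impact sound.
; At BeginPlay it passes its Name into the BP_PrintName widget.
; Each Tick turns that widget toward the player camera and shows it only while BPCanActionObjectDrawOutLine reports the object is watched.
; Plate hits play a dish sound at the actor's location when actor velocity reaches a small threshold.
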(event OnComponentHit(Plate)
  (params (HitComponent :type Primitive%20Component%20Object%20Reference) (OtherActor :type Actor%20Object%20Reference) (OtherComp :type Primitive%20Component%20Object%20Reference) (NormalImpulse :type Vector :default "0, 0, 0") (Hit :type Hit%20Result%20Structure%20%28by%20ref%29))
  (if (>= (Math|Vector|VectorLength (Transformation|GetVelocity)) 15.0)
    (Audio|PlaySoundatLocation "/Game/Scene/Audio/SE/SE_putDish.SE_putDish" (Transformation|GetActorLocation) "0, 0, 0" 1.0 1.0 0.0 0 0 0 0)))

(event EventBeginPlay
  (bind _asbp_print_name (Utilities|Casting|CastToBP_PrintName (UserInterface|GetWidget (Variables|Default|GetWidget))))
  (Variables|/Game/Scene/BruePrints/BP_PrintName.BP_PrintName_C|SetObjectName _asbp_print_name (Variables|Default|GetName)))

(event Collision|EventActorBeginOverlap
  (params (OtherActor :type Actor%20Object%20Reference)))

(event EventTick
  (params (DeltaSeconds :type Float%20%28single-precision%29))
  (Transformation|SetWorldRotation (Variables|Default|GetWidget) (Math|Rotator|FindLookatRotation (Transformation|GetWorldLocation (Variables|Default|GetWidget)) (Camera|GetCameraLocation (Game|GetPlayerCameraManager 0))) false false)
  (bind _iswatch (Default|GetIsWatch (Variables|Default|GetBP_CanActionObjectDrawOutLine)))
  (Development|SetHiddeninGame (Variables|Default|GetWidget) (not _iswatch) false))

(fn ConstructionScript)