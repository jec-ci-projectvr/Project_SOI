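; BP_Hall is a puzzle hall with three overlap-triggered buttons and a front wall that serves as a door.
; Each press advances that button's count modulo 8 and animates it along Y with its collision temporarily disabled.
; When the animation finishes, the button reports to the GameInstance whether its count matches its target.
; An OpenDoor interface event raises the wall on a timeline when it receives the matching mystery enum value.
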(event OnComponentBeginOverlap(Button0)
  (params (OverlappedComponent :type Primitive%20Component%20Object%20Reference) (OtherActor :type Actor%20Object%20Reference) (OtherComp :type Primitive%20Component%20Object%20Reference) (OtherBodyIndex :type Integer) (bFromSweep :type Boolean) (SweepResult :type Hit%20Result%20Structure%20%28by%20ref%29))
  ;[1 1 1] ボタンの当たり判定
  (CallFunction|OnButtonAction (Variables|Default|GetButton0)))

(event OnComponentBeginOverlap(Button1)
  (params (OverlappedComponent :type Primitive%20Component%20Object%20Reference) (OtherActor :type Actor%20Object%20Reference) (OtherComp :type Primitive%20Component%20Object%20Reference) (OtherBodyIndex :type Integer) (bFromSweep :type Boolean) (SweepResult :type Hit%20Result%20Structure%20%28by%20ref%29))
  ;[1 1 1] ボタンの当たり判定
  (CallFunction|OnButtonAction (Variables|Default|GetButton1) 1))

(event OnComponentBeginOverlap(Button2)
  (params (OverlappedComponent :type Primitive%20Component%20Object%20Reference) (OtherActor :type Actor%20Object%20Reference) (OtherComp :type Primitive%20Component%20Object%20Reference) (OtherBodyIndex :type Integer) (bFromSweep :type Boolean) (SweepResult :type Hit%20Result%20Structure%20%28by%20ref%29))
  ;[1 1 1] ボタンの当たり判定
  (CallFunction|OnButtonAction (Variables|Default|GetButton2) 2))

(event Custom|OnButtonAction
  (params (pushButton :type Primitive%20Component%20Object%20Reference) (Number :type Integer))
  (bind _beforebuttonposion (Variables|Default|GetbeforeButtonPosion))
  (bind _output (Utilities|Array|Get(acopy) _beforebuttonposion Number))
  ;[1 1 1] 指定回数ならフラグをＴｒｕｅ
  (bind _result (Math|Integer|IncrementInt (Utilities|Array|Get(acopy) (Variables|Default|Getcount) Number))
    (:%20%20
      (Utilities|Array|SetArrayElem (Variables|Default|Getcount) Number (Math|Integer|%(Integer) _result 8))
      (bind _button (Timeline|TimeLine PlayFromStart)
        (:Update
          (Transformation|SetWorldLocation pushButton (Math|Vector|MakeVector (.x _output) (- (.y _output) (* 1e+01 _button)) (.z _output)) false false)
          (Collision|SetCollisionEnabled pushButton "NoCollision"))
        (:Finished
          (Collision|SetCollisionEnabled pushButton "QueryAndPhysics")
          (Class|BPIEvent|ButtonHallFlg(Message) (Game|GetGameInstance) (== (Utilities|Array|Get(acopy) (Variables|Default|Getcount) Number) (Utilities|Array|Get(acopy) (Variables|Default|Getmax) Number)) Number))))))

(event Custom|CheckAndOpen
  (params (mystery :type MysteryPlace%20Enum :default "NewEnumerator0"))
  (bind _beforedoorposition (Variables|Default|GetbeforeDoorPosition))
  ;[1 1 1] サーバーから扉を開く
  (if (Utilities|Enum|Equal(Enum) mystery "NewEnumerator3")
    (bind _door (Timeline|DoorAnim Play)
      (:Update
        (Transformation|SetWorldLocation (Variables|Default|GetWall_Front) (Math|Vector|MakeVector (.x _beforedoorposition) (.y _beforedoorposition) (+ (.z _beforedoorposition) (* _door 3e+02))) false false)))))

(event EventBeginPlay
  (for (_ _array_index) (Variables|Default|GetbeforeButtonPosion)
    (bind _location (CallFunction|GetLocation _array_index))
    (Utilities|Array|SetArrayElem (Variables|Default|GetbeforeButtonPosion) _array_index _location)
    (Variables|Default|SetbeforeDoorPosition (Transformation|GetWorldLocation (Variables|Default|GetWall_Front)))))

(event Collision|EventActorBeginOverlap
  (params (OtherActor :type Actor%20Object%20Reference)))

(event EventTick
  (params (DeltaSeconds :type Float%20%28single-precision%29)))

(event EventOpenDoor
  (params (mystery :type MysteryPlace%20Enum :default "NewEnumerator0"))
  ;[1 1 1] インターフェースから受け取り
  (CallFunction|CheckandOpen mystery))

(fn ConstructionScript)

(fn GetLocation
  (params (num :type Integer))
  (switch int num
    (:0
      (return (Transformation|GetWorldLocation (Variables|Default|GetButton0))))
    (:1
      (return (Transformation|GetWorldLocation (Variables|Default|GetButton1))))
    (:2
      (return (Transformation|GetWorldLocation (Variables|Default|GetButton2))))))