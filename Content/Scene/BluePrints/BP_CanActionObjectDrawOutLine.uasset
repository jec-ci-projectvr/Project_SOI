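; BP_CanActionObjectDrawOutLine is a component that outlines its owner's static meshes when the object is near the camera's view center, signaling it can be acted on.
; Each Tick compares the dot product of camera forward and direction to the owner against Tolerance.
; Parent static mesh components get an M_Overlay outline above that threshold and lose it otherwise.
; A new dynamic material instance is created every passing frame.
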(event EventBeginPlay)

(event EventTick
  (params (DeltaSeconds :type Float%20%28single-precision%29))
  (bind _returnvalue (Game|GetPlayerCameraManager 0))
  ;[1 1 1] このコンポーネントの親で、スタティックメッシュであるものを全て変化
  (for _array_element (Class|SceneComponent|GetParentComponents)
    (bind _asstatic_mesh_component (Utilities|Casting|CastToStaticMeshComponent _array_element))
    ;;[0.3438 0 0.003011] アクション可能範囲内ならアウトラインを付ける、それ以外ならアウトラインを消す
    (if (> (Math|Vector|DotProduct (Transformation|GetActorForwardVector _returnvalue) (Math|Vector|Normalize (- (Transformation|GetActorLocation (Components|GetOwner)) (Camera|GetCameraLocation _returnvalue)))) (Variables|Default|Gettolerance))
      (bind _returnvalue_2 (Rendering|Material|CreateDynamicMaterialInstance "/Game/material/M_Overlay.M_Overlay" "None" "None" :!class /Script/Engine.KismetMaterialLibrary))
      (Rendering|Material|SetScalarParameterValue _returnvalue_2 "OutLineOffset" 0.5 :!class /Script/Engine.MaterialInstanceDynamic)
      (Rendering|Material|SetOverlayMaterial _asstatic_mesh_component _returnvalue_2 :!class /Script/Engine.MeshComponent)
      (else
        (Rendering|Material|SetOverlayMaterial _asstatic_mesh_component 0 :!class /Script/Engine.MeshComponent)))))