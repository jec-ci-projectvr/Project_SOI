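; BP_Door1 is a door actor that opens by jumping 300 units along world X when its linked triggers allow it.
; On BeginPlay it binds to the OnButtonDown dispatcher of BP_Button1 entries in the DoorFlag array.
; Each press runs CheckDoorFlag, which casts entries to BP_DoorTrigger and queries DoorFlagMessage, breaking on the first false.
; If none breaks the check, DoorTransForm moves the actor instantly and prints debug strings.
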(event Custom|OnButtonDown_Event
  (CallFunction|CheckDoorFlag))

(event Collision|EventActorBeginOverlap
  (params (OtherActor :type Actor%20Object%20Reference)))

(event EventTick
  (params (DeltaSeconds :type Float%20%28single-precision%29)))

(event EventBeginPlay
  (for _array_element (Variables|Default|GetdoorFlag)
    (bind _asbp_button_1 (Utilities|Casting|CastToBP_Button1 _array_element))
    (EventDispatchers|AssignOnButtonDown _asbp_button_1 (delegate Custom|OnButtonDown_Event))))

(fn ConstructionScript)

(fn CheckDoorFlag
  (bind _array_element (Utilities|Array|ForEachLoopwithBreak (Variables|Default|GetdoorFlag) :!label _label)
    (:LoopBody
      (bind _asbp_door_trigger (Utilities|Casting|CastToBP_DoorTrigger _array_element))
      (bind _flag (Class|BPDoorTrigger|DoorFlag(Message) (Utilities|ToObject(Interface) _asbp_door_trigger)))
      (if (not _flag)
        (LocalVariables|SetisBreak true)
        (goto _label Break)))
    (:Completed
      (if (not (LocalVariables|GetisBreak))
        (Development|PrintString "Hello")
        (CallFunction|DoorTransForm)))))

(fn DoorTransForm
  (bind _returnvalue (Transformation|GetActorLocation))
  (Development|PrintString "Door Open")
  (Transformation|SetActorLocation (Math|Vector|MakeVector (+ (.x _returnvalue) 3e+02) (.y _returnvalue) (.z _returnvalue)) false false)
  (Development|PrintString "MOVE! MOVED! MOVED! "))