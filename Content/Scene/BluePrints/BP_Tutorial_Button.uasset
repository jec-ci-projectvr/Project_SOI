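; Tutorial push button that counts overlaps with its Button component, wrapping the count at ten, and plays a sound on each press.
; A timeline animates the actor along world Y from its start position, disabling the button's collision during the movement.
; A timeline event writes the count to the BP_ButtonPrintNumber widget.
; On finish, collision returns and the GameInstance receives the button number and whether the count equals PushMax.
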(event OnComponentBeginOverlap(Button)
  (params (OverlappedComponent :type Primitive%20Component%20Object%20Reference) (OtherActor :type Actor%20Object%20Reference) (OtherComp :type Primitive%20Component%20Object%20Reference) (OtherBodyIndex :type Integer) (bFromSweep :type Boolean) (SweepResult :type Hit%20Result%20Structure%20%28by%20ref%29))
  (bind _beforeposition (Variables|Default|GetbeforePosition))
  (bind _result (Math|Integer|IncrementInt (Variables|Default|GetpushCnt))
    (:%20%20
      (Variables|Default|SetpushCnt (Math|Integer|%(Integer) _result 10))
      (Audio|PlaySoundatLocation 0 (Variables|Default|GetbeforePosition) "0, 0, 0" 1.0 1.0 0.0 0 0 0 0)
      (bind _button (Timeline|Timeline PlayFromStart)
        (:Update
          (Transformation|SetActorLocation (Math|Vector|MakeVector (.x _beforeposition) (+ (.y _beforeposition) (* 1e+01 _button)) (.z _beforeposition)) false false)
          (Collision|SetCollisionEnabled (Variables|Default|GetButton) "NoCollision"))
        (:Finished
          (Collision|SetCollisionEnabled (Variables|Default|GetButton) "QueryAndPhysics")
          (Class|BPIEvent|ButtonTutrialFlg(Message) (Game|GetGameInstance) (== (Variables|Default|GetpushCnt) (Variables|Default|GetpushMax)) (Variables|Default|GetbuttonNum)))
        (:Widget
          (bind _asbp_button_print_number (Utilities|Casting|CastToBP_ButtonPrintNumber (UserInterface|GetUserWidgetObject (Variables|Default|GetWidget))))
          (Variables|/Game/Scene/BruePrints/BP_ButtonPrintNumber.BP_ButtonPrintNumber_C|SetNewVar_0 _asbp_button_print_number (Variables|Default|GetpushCnt)))))))

(event EventBeginPlay
  (Variables|Default|SetbeforePosition (Transformation|GetActorLocation)))

(event Collision|EventActorBeginOverlap
  (params (OtherActor :type Actor%20Object%20Reference)))

(event EventTick
  (params (DeltaSeconds :type Float%20%28single-precision%29)))

(fn ConstructionScript)