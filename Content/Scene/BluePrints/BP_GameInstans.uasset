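; Game instance for a two-player LAN VR puzzle game, handling sessions and puzzle progress.
; Hosts VRTemplateMap as a listen server or joins the first session found.
; Tutorial button, statue, hall button, dining and chess events update per-puzzle arrays; CheckFlg marks fully solved puzzles cleared once and sends OpenDoorMessage to all BPI_Event actors.
; StartGame resets all flag arrays through nested loops.
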(event Custom|StartGame
  (bind _statuecomplate (Variables|Default|GetstatueComplate))
  (bind _tutrialbuttoncomplate (Variables|Default|GettutrialButtonComplate))
  (bind _chesscomplate (Variables|Default|GetChessComplate))
  (bind _dinningcomplate (Variables|Default|GetDinningComplate))
  (bind _hallbuttoncomplate (Variables|Default|GethallButtonComplate))
  (bind _isclear (Variables|Default|GetisClear))
  (for (_ _array_index) _isclear
    (Utilities|Array|SetArrayElem _isclear _array_index false)
    (for (_ _array_index_2) _tutrialbuttoncomplate
      (Utilities|Array|SetArrayElem _tutrialbuttoncomplate _array_index_2 false)
      (for (_ _array_index_3) _statuecomplate
        (Utilities|Array|SetArrayElem _statuecomplate _array_index_3 false)
        (for (_ _array_index_4) _hallbuttoncomplate
          (Utilities|Array|SetArrayElem _hallbuttoncomplate _array_index_4 false)
          (for (_ _array_index_5) _dinningcomplate
            (Utilities|Array|SetArrayElem _dinningcomplate _array_index_5 false)
            (for (_ _array_index_6) _chesscomplate
              (Utilities|Array|SetArrayElem _chesscomplate _array_index_6 false))))))))

(event Custom|CheckFlg
  (params (useArray :type Array%20of%20Booleans) (mystery :type MysteryPlace%20Enum :default "NewEnumerator0"))
  (bind _returnvalue (Math|Conversions|ToInteger(Byte) mystery))
  ;[1 1 1] 全て正解したら扉を開く
  (if (not (Utilities|Array|Get(acopy) (Variables|Default|GetisClear) _returnvalue))
    (Variables|Default|Setcheck true)
    (bind _array_element (Utilities|Array|ForEachLoopwithBreak useArray :!label _label)
      (:LoopBody
        (if (not (== _array_element true))
          (Variables|Default|Setcheck false)
          (goto _label Break)))
      (:Completed
        (if (Variables|Default|Getcheck)
          (Utilities|Array|SetArrayElem (Variables|Default|GetisClear) _returnvalue true)
          (bind _outactors (Actor|GetAllActorswithInterface "/Game/Scene/BluePrints/BPI_Event.BPI_Event_C"))
          (for _array_element_2 _outactors
            (Class|BPIEvent|OpenDoor(Message) _array_element_2 mystery)))))))

(event EventButtonHallFlg
  (params (condition :type Boolean) (buttonNum :type Integer))
  (bind _hallbuttoncomplate (Variables|Default|GethallButtonComplate))
  ;[1 1 1] インターフェースを受け取りサーバーで実行
  (Utilities|Array|SetArrayElem _hallbuttoncomplate buttonNum condition)
  (CallFunction|CheckFlg _hallbuttoncomplate "NewEnumerator3"))

(event EventObjectFlg
  (params (condition :type Boolean) (dishNum :type Integer))
  (bind _dinningcomplate (Variables|Default|GetDinningComplate))
  ;[1 1 1] インターフェースを受け取りサーバーで実行
  (Utilities|Array|SetArrayElem _dinningcomplate dishNum condition)
  (CallFunction|CheckFlg _dinningcomplate "NewEnumerator1"))

(event EventFindSession
  (bind _returnvalue (Game|GetPlayerController 0))
  ;[1 1 1] セッションを探して入る
  (bind _results (|FindSessions _returnvalue 100 true)
    (:then
      (Development|PrintString "Looking for available sessions to attend." true true "(R=0.000000,G=1.000000,B=0.000000,A=1.000000)" 5.0))
    (:OnSuccess
      (if (> (Utilities|Array|Length _results) 0)
        (|JoinSession _returnvalue (Utilities|Array|Get(acopy) _results)
          (:OnSuccess
            (Development|PrintString "OK_Client_Join" true true "(R=0.000000,G=0.000000,B=1.000000,A=1.000000)")))))))

(event EventChessFlg
  (params (condition :type Boolean) (chessNum :type Integer))
  (bind _chesscomplate (Variables|Default|GetChessComplate))
  ;[1 1 1] インターフェースを受け取りサーバーで実行
  (Utilities|Array|SetArrayElem _chesscomplate chessNum condition)
  (CallFunction|CheckFlg _chesscomplate "NewEnumerator2"))

(event EventMakeSession
  ;[1 1 1] セッションを作成
  (|Session (Game|GetPlayerController 0) 2 true
    (:OnSuccess
      (Game|OpenLevel(byName) "VRTemplateMap" true "?listen")
      (Development|PrintString "OK_Session_Create" true true "(R=0.000000,G=0.000000,B=1.000000,A=1.000000)"))))

(event EventButtonTutrialFlg
  (params (condition :type Boolean) (buttonNum :type Integer))
  (bind _tutrialbuttoncomplate (Variables|Default|GettutrialButtonComplate))
  ;[1 1 1] インターフェースを受け取りサーバーで実行
  (Utilities|Array|SetArrayElem _tutrialbuttoncomplate buttonNum condition)
  (CallFunction|CheckFlg _tutrialbuttoncomplate "NewEnumerator0"))

(event EventStatueFlg
  (params (condition :type Boolean) (statueNum :type Integer))
  (bind _statuecomplate (Variables|Default|GetstatueComplate))
  ;[1 1 1] インターフェースを受け取りサーバーで実行
  (Utilities|Array|SetArrayElem _statuecomplate statueNum condition)
  (CallFunction|CheckFlg _statuecomplate "NewEnumerator4"))