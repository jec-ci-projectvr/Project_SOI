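; BP_Button is a pushable button that counts its presses and reports to the game instance whether its target count is met.
; Each overlap on the Button component increments a counter that wraps at eight and plays a timeline sliding the actor along Y from its start position.
; Collision is off during the animation; on finish it is restored and ButtonFlgMessage receives the button number and completion flag.
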(event OnComponentBeginOverlap(Button)
  (params (OverlappedComponent :type Primitive%20Component%20Object%20Reference) (OtherActor :type Actor%20Object%20Reference) (OtherComp :type Primitive%20Component%20Object%20Reference) (OtherBodyIndex :type Integer) (bFromSweep :type Boolean) (SweepResult :type Hit%20Result%20Structure%20%28by%20ref%29))
  (bind _currentposition (Variables|Default|GetCurrentPosition))
  (bind _result (Math|Integer|IncrementInt (Variables|Default|GetpushCnt))
    (:%20%20
      (Variables|Default|SetpushCnt (Math|Integer|%(Integer) _result 8))
      (bind _newtrack_0 (Timeline|Timeline PlayFromStart)
        (:Update
          (Transformation|SetActorLocation (Math|Vector|MakeVector (.x _currentposition) (- (.y _currentposition) (* 1e+01 _newtrack_0)) (.z _currentposition)) false false)
          (Collision|SetCollisionEnabled (Variables|Default|GetButton) "NoCollision"))
        (:Finished
          (Collision|SetCollisionEnabled (Variables|Default|GetButton) "QueryAndPhysics")
          (Class|BPIEvent|ButtonFlg(Message) (Game|GetGameInstance) (== (Variables|Default|GetpushCnt) (Variables|Default|GetpushMax)) (Variables|Default|GetbuttonNum)))))))

(event EventBeginPlay
  (Variables|Default|SetCurrentPosition (Transformation|GetActorLocation)))

(event Collision|EventActorBeginOverlap
  (params (OtherActor :type Actor%20Object%20Reference)))

(event EventTick
  (params (DeltaSeconds :type Float%20%28single-precision%29)))

(fn ConstructionScript)