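; BP_Statue1 is a statue actor that a trigger button rotates, likely as part of a puzzle.
; On BeginPlay it binds to the TriggerButton's OnButtonDown dispatcher.
; Each press sets the statue's yaw in 45-degree steps from the received count and sets StatueFlag when that count equals PushCnt.
; A debug string prints on every press.
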(event Custom|OnButtonDown_Event
  (params (inCnt :type Integer))
  (Development|PrintString "Hello")
  (Variables|Default|SetstatueFlag (== inCnt (Variables|Default|GetpushCnt)))
  (Transformation|SetActorRotation (Math|Rotator|MakeRotator 0.0 0.0 (Math|Conversions|ToFloat(Integer) (* inCnt 45)))))

(event EventBeginPlay
  (EventDispatchers|BindEventtoOnButtonDown (Variables|Default|GettriggerButton) (delegate Custom|OnButtonDown_Event)))

(event Collision|EventActorBeginOverlap
  (params (OtherActor :type Actor%20Object%20Reference)))

(event EventTick
  (params (DeltaSeconds :type Float%20%28single-precision%29)))

(fn ConstructionScript)