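; BP_Door is a double-door actor that swings open in response to an OpenDoor interface call carrying a Mystery value.
; BeginPlay caches the starting world rotation of both door panels.
; OpenDoor forwards to CheckAndOpen, commented as server-side, which compares Mystery values and plays the DoorAnimation timeline on a match.
; The timeline offsets each panel's cached yaw in opposite directions, up to a quarter turn at full value.
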(event Custom|CheckAndOpen
  (params (mystery :type MysteryPlace%20Enum :default "NewEnumerator0"))
  (bind _beforeright (Variables|Default|GetbeforeRight))
  (bind _beforeleft (Variables|Default|GetbeforeLeft))
  ;[1 1 1] サーバーから扉を開く
  (if (Utilities|Enum|Equal(Enum) mystery (Variables|Default|Getmystery))
    (bind _door (Timeline|DoorAnimation Play)
      (:Update
        (Transformation|SetWorldRotation (Variables|Default|GetRightDoor) (Math|Rotator|MakeRotator (.roll _beforeright) (.pitch _beforeright) (+ (.yaw _beforeright) (* _door 9e+01))) false false)
        (Transformation|SetWorldRotation (Variables|Default|GetLeftDoor) (Math|Rotator|MakeRotator (.roll _beforeleft) (.pitch _beforeleft) (+ (.yaw _beforeleft) (* _door -9e+01))) false false)))))

(event EventOpenDoor
  (params (mystery :type MysteryPlace%20Enum :default "NewEnumerator0"))
  ;[1 1 1] インターフェースから受け取り
  (CallFunction|CheckandOpen mystery))

(event Collision|EventActorBeginOverlap
  (params (OtherActor :type Actor%20Object%20Reference)))

(event EventTick
  (params (DeltaSeconds :type Float%20%28single-precision%29)))

(event EventBeginPlay
  ;[1 1 1] 最初の位置を取得
  (Variables|Default|SetbeforeRight (Transformation|GetWorldRotation (Variables|Default|GetRightDoor)))
  (Variables|Default|SetbeforeLeft (Transformation|GetWorldRotation (Variables|Default|GetLeftDoor))))

(fn ConstructionScript)