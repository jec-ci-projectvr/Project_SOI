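; BP_SceneChange is a trigger actor that hands off from gameplay to a sequence when the player enters its box.
; On overlap by the player character, it disables that character's input and fades the camera and audio to black, holding the fade.
; After a delay matching the fade duration, it plays the sequence referenced by Movie.
; The Blueprint itself neither restores input nor loads a level.
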(event OnComponentBeginOverlap(Box)
  (params (OverlappedComponent :type Primitive%20Component%20Object%20Reference) (OtherActor :type Actor%20Object%20Reference) (OtherComp :type Primitive%20Component%20Object%20Reference) (OtherBodyIndex :type Integer) (bFromSweep :type Boolean) (SweepResult :type Hit%20Result%20Structure%20%28by%20ref%29))
  ;[1 1 1] トリガーに入ったアクターがプレイヤーなら
  (if (== OtherActor (Game|GetPlayerCharacter 0))
    ;[1 1 1] 入力を止める
    (Input|DisableInput OtherActor (Game|GetPlayerController 0))
    ;[1 1 1] 暗転
    (CameraFades|StartCameraFade (Game|GetPlayerCameraManager 0) 0.0 1.0 3.0 "(R=0.000000,G=0.000000,B=0.000000,A=1.000000)" true true)
    (Utilities|FlowControl|Delay 3.0)
    (Sequencer|Player|Play (Variables|/Script/LevelSequence.LevelSequenceActor|GetSequencePlayer (Variables|Default|Getmovie)) :!class /Script/MovieScene.MovieSceneSequencePlayer)))

(event EventBeginPlay)

(event Collision|EventActorBeginOverlap
  (params (OtherActor :type Actor%20Object%20Reference)))

(event EventTick
  (params (DeltaSeconds :type Float%20%28single-precision%29)))

(fn ConstructionScript)